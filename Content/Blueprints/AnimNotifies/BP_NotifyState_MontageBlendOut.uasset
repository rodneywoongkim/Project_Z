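; Anim notify state that blends a character's montage out early while its window is active, once a chosen condition is met.
; Each tick it evaluates the BlendOutCondition enum: forced, movement input or its absence, falling, acceleration, or input axes read through an interface call on the character.
; An optional crouch check can also interrupt, and all paths stop the montage with BlendOutTime.
; The notify's display name includes the selected condition.
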(fn `GetNotifyName`
  (returns (ReturnValue :type String))
  (return (`KismetStringLibrary.Concat_StrStr` "Early Blend out - " (`|GetEnumeratorNameAsString` (`self.BlendOutCondition`)))))

(fn `Received_NotifyTick`
  (params (MeshComp :type "SkeletalMeshComponent Object Reference") (Animation :type "AnimSequenceBase Object Reference") (FrameDeltaTime :type "Float (single-precision)") (EventReference :type "AnimNotifyEventReference Structure (by ref)"))
  (returns (ReturnValue :type Boolean))
  (locals (Character :type "Character Object Reference") (AnimInstance :type "AnimInstance Object Reference") (AnimMontage :type "AnimMontage Object Reference"))
  (bind _ascharacter (cast `Character` (`ActorComponent.GetOwner` (`local.MeshComp`))))
  (set `local.Character` _ascharacter)
  (set `local.AnimInstance` (`SkeletalMeshComponent.GetAnimInstance` (`local.MeshComp`)))
  (bind _asanim_montage (cast `AnimMontage` (`local.Animation`)))
  (set `local.AnimMontage` _asanim_montage)
  (`|ExecutionSequence`
    (:`then_0`
      (switch `/Game/AdvancedLocomotionV4/Data/Enums/E_TraversalBlendOutCondition` (`self.BlendOutCondition`)
        (:`NewEnumerator0`
          (`AnimInstance.Montage_Stop` (`local.AnimInstance`) (`self.BlendOutTime`) (`local.AnimMontage`))
          (return true))
        (:`NewEnumerator1`
          (if (!= (`PawnMovementComponent.GetLastInputVector` (`Character.CharacterMovement` (`local.Character`))) (0.0 0.0 0.0) :`ErrorTolerance` 0.1)
            (`AnimInstance.Montage_Stop` (`local.AnimInstance`) (`self.BlendOutTime`) (`local.AnimMontage`))
            (return true)))
        (:`NewEnumerator2`
          (if (`NavMovementComponent.IsFalling` (`Character.CharacterMovement` (`local.Character`)))
            (`AnimInstance.Montage_Stop` (`local.AnimInstance`) (`self.BlendOutTime`) (`local.AnimMontage`))
            (return true)))
        (:`NewEnumerator3`
          (if (== (`PawnMovementComponent.GetLastInputVector` (`Character.CharacterMovement` (`local.Character`))) (0.0 0.0 0.0) :`ErrorTolerance` 0.1)
            (`AnimInstance.Montage_Stop` (`local.AnimInstance`) (`self.BlendOutTime`) (`local.AnimMontage`))
            (return true)))
        (:`NewEnumerator4`
          (if (> (`KismetMathLibrary.VSize` (`CharacterMovementComponent.GetCurrentAcceleration` (`Character.CharacterMovement` (`local.Character`)))) 20.0)
            (`AnimInstance.Montage_Stop` (`local.AnimInstance`) (`self.BlendOutTime`) (`local.AnimMontage`))
            (return true)))
        (:`NewEnumerator5`
          (bind (_move_forward_axis _move_right_axis) (message `/Game/AdvancedLocomotionV4/Blueprints/Interfaces/ALS_Character_BPI.BPI_GetCharactersInputsAxis` (`local.Character`)))
          (if (or (!= _move_forward_axis 0.0) (!= _move_right_axis 0.0))
            (`AnimInstance.Montage_Stop` (`local.AnimInstance`) (`self.BlendOutTime`) (`local.AnimMontage`))
            (return true)))))
    (:`then_1`
      (if (`self.InterruptWhenCrouch`)
        (if (`Character.bIsCrouched` (`local.Character`))
          (`AnimInstance.Montage_Stop` (`local.AnimInstance`) (`self.BlendOutTime`) (`local.AnimMontage`))
          (return true))))))